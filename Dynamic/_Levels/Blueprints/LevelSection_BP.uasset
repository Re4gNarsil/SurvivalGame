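; Level section actor for a survival mode with endlessly spawned areas, gated by a red/green barrier that blocks or passes pawns.
; The player entering the Lock volume raises the level and opens the barrier; leaving shifts the NavMeshBoundsVolume forward, requests a new section from the game mode and locks it.
; CheckForAnyGuards opens the barrier when none remain.
; The Destruct trigger destroys actors inside Lock and the section itself.
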(event `CheckForAnyGuards`
  (bind _barrier (`self.Barrier`))
  (bind _returnvalue (`self.CheckForGuards` (`self.Lock`)))
  (if (not _returnvalue)
    ;[1 1 1] Enable/Disable Pawns Through Barriers
    (`PrimitiveComponent.SetCollisionResponseToChannel` _barrier "ECC_Pawn" "ECR_Ignore" :!label _label)
    (`PrimitiveComponent.SetMaterial` _barrier 0 "/Game/Static/_Levels/BarrierGreen.BarrierGreen")))

(event `self.Lock.OnComponentBeginOverlap`
  (params (OverlappedComponent :type "PrimitiveComponent Object Reference") (OtherActor :type "Actor Object Reference") (OtherComp :type "PrimitiveComponent Object Reference") (OtherBodyIndex :type Integer) (bFromSweep :type Boolean) (SweepResult :type "HitResult Structure (by ref)"))
  ;[1 1 1] Check to make sure the player is leaving/entering an area
  (bind _isplayer (`self.CheckActor` OtherActor))
  (if _isplayer
    (`self.PlayerUIUpdate` OtherActor)
    (goto _label)))

(event `self.ReceiveBeginPlay`
  ;[1 1 1] Enable/Disable Pawns Through Barriers
  (goto _label))

(event `LockBarrier`
  (bind _barrier (`self.Barrier`))
  ;[1 1 1] Enable/Disable Pawns Through Barriers
  (`PrimitiveComponent.SetCollisionResponseToChannel` _barrier "ECC_Pawn" "ECR_Block" :!label _label_2)
  (`PrimitiveComponent.SetMaterial` _barrier 0 "/Game/Static/_Levels/BarrierRed.BarrierRed"))

(event `self.Lock.OnComponentEndOverlap`
  (params (OverlappedComponent :type "PrimitiveComponent Object Reference") (OtherActor :type "Actor Object Reference") (OtherComp :type "PrimitiveComponent Object Reference") (OtherBodyIndex :type Integer))
  ;[1 1 1] Check to make sure the player is leaving/entering an area
  (bind _isplayer (`self.CheckActor` OtherActor))
  (if _isplayer
    (`self.ShiftNavMesh`)
    (`self.AddNewSection`)
    (goto _label_2)))

(event `self.Destruct.OnComponentBeginOverlap`
  (params (OverlappedComponent :type "PrimitiveComponent Object Reference") (OtherActor :type "Actor Object Reference") (OtherComp :type "PrimitiveComponent Object Reference") (OtherBodyIndex :type Integer) (bFromSweep :type Boolean) (SweepResult :type "HitResult Structure (by ref)"))
  (bind _overlappingactors (`PrimitiveComponent.GetOverlappingActors` (`self.Lock`) null))
  ;[1 1 1] Destroy this section and everything in it
  (bind _isplayer (`self.CheckActor` OtherActor))
  (if _isplayer
    (if (`KismetArrayLibrary.Array_IsValidIndex` _overlappingactors)
      (for _array_element _overlappingactors
        (`self.K2_DestroyActor` _array_element)))
    (`self.K2_DestroyActor`)))

(fn `AddNewSection`
  (bind _assurvival_game_game_mode_bp (cast `/Game/SurvivalGameGameMode_BP` (`GameplayStatics.GetGameMode`))
    (:`then`
      (`/Game/SurvivalGameGameMode_BP.SpawnNewSection` _assurvival_game_game_mode_bp))
    (:`CastFailed`
      _))
  (return))

(fn `CheckActor`
  (params (A :type "Object Object Reference"))
  (returns (IsPlayer :type Boolean))
  (locals (AmPlayer :type Boolean))
  (return (== A (`GameplayStatics.GetPlayerCharacter` 0))))

(fn `PlayerUIUpdate`
  (params (self2 :type "Actor Object Reference"))
  (bind _level (`self.Level`))
  (`KismetSystemLibrary.PrintString` (`KismetStringLibrary.Conv_IntToString` _level))
  (set `self.Level` (+ _level 1))
  (bind _asbp_my_player_controller (cast `/Game/Dynamic/FirstPerson/Blueprints/BP_MyPlayerController` (`Pawn.GetController` (`Actor.Instigator` self2)))
    (:`then`
      (`/Game/Dynamic/FirstPerson/Blueprints/BP_MyPlayerController.IncreaseLevel` _asbp_my_player_controller))
    (:`CastFailed`
      _))
  (return))

(fn `ShiftNavMesh`
  (bind _outactors (`GameplayStatics.GetAllActorsOfClass` "/Script/Engine.NavMeshBoundsVolume"))
  (bind _item (`KismetArrayLibrary.Array_Get` _outactors))
  (`self.K2_SetActorLocation` _item (+ (`self.K2_GetActorLocation` _item) (4000.0 0.0 0.0)) false false)
  (return))

(fn `UserConstructionScript`)